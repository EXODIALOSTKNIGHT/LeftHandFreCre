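; BP_GreenBox is a health pickup that triggers when a ThirdPersonCharacter overlaps its Box component.
; On overlap it spawns an explosion particle at its location, destroys itself, then adds a fixed amount to the character's Health.
; The maximum is only an exact-equality check that prints "max life", so other values are not clamped and the new Health is printed.
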(event `self.Box.OnComponentBeginOverlap`
  (params (OverlappedComponent :type "PrimitiveComponent Object Reference") (OtherActor :type "Actor Object Reference") (OtherComp :type "PrimitiveComponent Object Reference") (OtherBodyIndex :type Integer) (bFromSweep :type Boolean) (SweepResult :type "HitResult Structure (by ref)"))
  (bind _asthird_person_character (cast `/Game/ThirdPersonBP/Blueprints/ThirdPersonCharacter` OtherActor))
  (`GameplayStatics.SpawnEmitterAtLocation` "/Game/ParticleEffect/Particles/P_Explosion.P_Explosion" (`self.K2_GetActorLocation`))
  (`self.K2_DestroyActor`)
  (if (== (`/Game/ThirdPersonBP/Blueprints/ThirdPersonCharacter.Health` _asthird_person_character) 100.0)
    (set `/Game/ThirdPersonBP/Blueprints/ThirdPersonCharacter.Health` 100.0 _asthird_person_character)
    (`KismetSystemLibrary.PrintString` "max life")
    (else
      (bind _output_get (set `/Game/ThirdPersonBP/Blueprints/ThirdPersonCharacter.Health` (+ (`/Game/ThirdPersonBP/Blueprints/ThirdPersonCharacter.Health` _asthird_person_character) 20.0) _asthird_person_character))
      (`KismetSystemLibrary.PrintString` (`KismetStringLibrary.Conv_DoubleToString` _output_get)))))

(fn `UserConstructionScript`)