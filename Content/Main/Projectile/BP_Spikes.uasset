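; BP_Spikes is a short-lived projectile actor that explodes on contact with the colored box actors.
; Its Sphere1 overlap runs a cast for each box type: red and white boxes are destroyed, while violet and black boxes survive.
; All four box types destroy the spikes and spawn an explosion emitter at their location.
; Without such a hit, a BeginPlay delay removes the actor after under a second.
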(event `self.Sphere1.OnComponentBeginOverlap`
  (params (OverlappedComponent :type "PrimitiveComponent Object Reference") (OtherActor :type "Actor Object Reference") (OtherComp :type "PrimitiveComponent Object Reference") (OtherBodyIndex :type Integer) (bFromSweep :type Boolean) (SweepResult :type "HitResult Structure (by ref)"))
  (`|ExecutionSequence`
    (:`then_0`
      (bind _asbp_red_box (cast `/Game/Main/Objects/BP_RedBox` OtherActor))
      (`self.K2_DestroyActor` _asbp_red_box)
      (`self.K2_DestroyActor`)
      (`GameplayStatics.SpawnEmitterAtLocation` "/Game/ParticleEffect/Particles/P_Explosion.P_Explosion" (`self.K2_GetActorLocation`)))
    (:`then_1`
      (bind _asbp_white_box (cast `/Game/Main/Objects/BP_WhiteBox` OtherActor))
      (`self.K2_DestroyActor` _asbp_white_box)
      (`self.K2_DestroyActor`)
      (`GameplayStatics.SpawnEmitterAtLocation` "/Game/ParticleEffect/Particles/P_Explosion.P_Explosion" (`self.K2_GetActorLocation`)))
    (:`then_2`
      (cast `/Game/Main/Objects/BP_VioletBox` OtherActor)
      (`self.K2_DestroyActor`)
      (`GameplayStatics.SpawnEmitterAtLocation` "/Game/ParticleEffect/Particles/P_Explosion.P_Explosion" (`self.K2_GetActorLocation`)))
    (:`then_3`
      (cast `/Game/Main/Objects/BP_BlackBox` OtherActor)
      (`self.K2_DestroyActor`)
      (`GameplayStatics.SpawnEmitterAtLocation` "/Game/ParticleEffect/Particles/P_Explosion.P_Explosion" (`self.K2_GetActorLocation`)))))

(event `self.ReceiveBeginPlay`
  (`KismetSystemLibrary.Delay` 0.7)
  (`self.K2_DestroyActor`))

(fn `UserConstructionScript`)